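; BP_BreakableTile is a ceiling tile prop that drops when its collision box is overlapped, then resets itself.
; Any overlap enables physics simulation on the tile mesh, with no check on the overlapping actor.
; After a ten-second delay, ResetProp disables physics and teleports the mesh to the location saved at BeginPlay.
; Only location is saved, so the reset does not restore a saved rotation.
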(event OnComponentBeginOverlap(CollisionBox)
  (params (OverlappedComponent :type Primitive%20Component%20Object%20Reference) (OtherActor :type Actor%20Object%20Reference) (OtherComp :type Primitive%20Component%20Object%20Reference) (OtherBodyIndex :type Integer) (bFromSweep :type Boolean) (SweepResult :type Hit%20Result%20Structure%20%28by%20ref%29))
  (Physics|SetSimulatePhysics (Variables|Default|GetSM_CeilingTile) true)
  (Utilities|FlowControl|Delay 1e+01)
  (CallFunction|ResetProp))

(event Custom|ResetProp
  (Physics|SetSimulatePhysics (Variables|Default|GetSM_CeilingTile) false)
  (Transformation|SetWorldLocationAndRotation (Variables|Default|GetSM_CeilingTile) (Variables|Default|GetStartingPos) "0, 0, 0" false true))

(event EventBeginPlay
  (Variables|Default|SetStartingPos (Transformation|GetWorldLocation (Variables|Default|GetSM_CeilingTile))))

(fn ConstructionScript)